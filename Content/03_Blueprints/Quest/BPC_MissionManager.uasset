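; Mission manager component that tracks active quests and advances them through Move to and Interact steps, reporting progress with PrintString.
; Each new step binds to SphereToGo or BP_InteractionBase actors with a matching Id and activates BPI_QuestActivatable actors it lists.
; Goal events match the first quest expecting that action and Id, then increment its count.
; A completed step unbinds its goals, then starts the next or removes the finished quest.
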(event `NextStep`
  (params (QuestStep :type "/Game/03_Blueprints/Quest/SQuestStep Structure"))
  (bind ((`TextForPlayer_7_0AF38C0D4441331E1301D69330518E34` _textforplayer) (`IdsToActivate_12_5EDD01BB4C040ACE0A12B792024F330E` _idstoactivate)) (break `/Game/03_Blueprints/Quest/SQuestStep` QuestStep))
  (`self.BindStep` QuestStep)
  (bind _outactors (`GameplayStatics.GetAllActorsWithInterface` "/Game/03_Blueprints/Quest/BPI_QuestActivatable.BPI_QuestActivatable_C"))
  (for _array_element _outactors
    (bind _id (message `/Game/03_Blueprints/Quest/BPI_QuestActivatable.GetActivatableId` _array_element))
    (if (`KismetArrayLibrary.Array_Contains` _idstoactivate _id)
      (message `/Game/03_Blueprints/Quest/BPI_QuestActivatable.Activate` _array_element)))
  (`KismetSystemLibrary.PrintString` (`KismetStringLibrary.Concat_StrStr` "New Task :" _textforplayer) true true (struct :`R` 0.121739 :`G` 1.0 :`B` 0.243927 :`A` 1.0) 5.0))

(event `BindStep`
  (params (Step :type "/Game/03_Blueprints/Quest/SQuestStep Structure"))
  (bind ((`Type_2_86DC646144700A12C04818AA1D21B893` _type) (`Id_5_617C013D4E997D033E706682BD127BB1` _id)) (break `/Game/03_Blueprints/Quest/SQuestStep` Step))
  (switch `/Game/03_Blueprints/Quest/EActionType` _type
    (:`NewEnumerator0`
      (bind _spherestogo (`self.FindMoveToGoal` _id))
      (for _array_element _spherestogo
        (add `/Game/03_Blueprints/Quest/SphereToGo.OnReachedByPlayer` _array_element (delegate `MoveTo`))))
    (:`NewEnumerator1`
      (bind _spherestogo_2 (`self.FindInteractGoal` _id))
      (for _array_element_2 _spherestogo_2
        (add `/Game/03_Blueprints/BP_InteractionBase.OnInteracted` _array_element_2 (delegate `Interact`))))))

(event `MoveTo`
  (params (Id :type String))
  (bind (_expected _questindex) (`self.ActionIdIsExpected` "NewEnumerator0" Id))
  (if _expected
    (bind _output_get (set `self.CurrentQuest` _questindex))
    (bind _finished (`self.ProgressQuest` _output_get))
    (if _finished
      (`self.FinishQuest` (`self.CurrentQuest`) :!label _label))))

(event `Interact`
  (params (Id :type String))
  (bind (_expected _questindex) (`self.ActionIdIsExpected` "NewEnumerator1" Id))
  (if _expected
    (bind _output_get (set `self.CurrentQuest` _questindex))
    (bind _finished (`self.ProgressQuest` _output_get))
    (if _finished
      (goto _label))))

(event `UnbindStep`
  (params (Step :type "/Game/03_Blueprints/Quest/SQuestStep Structure"))
  (bind ((`Type_2_86DC646144700A12C04818AA1D21B893` _type) (`Id_5_617C013D4E997D033E706682BD127BB1` _id)) (break `/Game/03_Blueprints/Quest/SQuestStep` Step))
  (switch `/Game/03_Blueprints/Quest/EActionType` _type
    (:`NewEnumerator0`
      (bind _spherestogo (`self.FindMoveToGoal` _id))
      (for _array_element _spherestogo
        (remove `/Game/03_Blueprints/Quest/SphereToGo.OnReachedByPlayer` _array_element (delegate `MoveTo`))))
    (:`NewEnumerator1`
      (bind _spherestogo_2 (`self.FindInteractGoal` _id))
      (for _array_element_2 _spherestogo_2
        (remove `/Game/03_Blueprints/BP_InteractionBase.OnInteracted` _array_element_2 (delegate `Interact`))))))

(event `AddNewQuest`
  (params (Quest :type "/Game/03_Blueprints/Quest/BP_DA_Quest Object Reference"))
  (bind _output (`|GetArrayItem` (`/Game/03_Blueprints/Quest/BP_DA_Quest.Steps` Quest)))
  (`KismetArrayLibrary.Array_Add` (`self.Quests`) (make `/Game/03_Blueprints/Quest/SQuestWrapper` Quest 0 _output))
  (`KismetSystemLibrary.PrintString` (`KismetStringLibrary.Concat_StrStr` "You started :" (`/Game/03_Blueprints/Quest/BP_DA_Quest.QuestName` Quest)) true true (struct :`R` 1.0 :`G` 0.603889 :`B` 0.003424 :`A` 1.0) 10.0)
  (`self.NextStep` _output))

(event `FinishQuest`
  (params (QuestIndex :type Integer))
  (`KismetSystemLibrary.PrintString` (`KismetStringLibrary.Concat_StrStr` "You have completed :" (`/Game/03_Blueprints/Quest/BP_DA_Quest.QuestName` (`.Quest_2_76C9A64A4DA53359FCA3478024055A09` (break `/Game/03_Blueprints/Quest/SQuestWrapper` (`|GetArrayItem` (`self.Quests`) QuestIndex))))) true true (struct :`R` 1.0 :`G` 0.603889 :`B` 0.003424 :`A` 1.0) 10.0)
  (`KismetArrayLibrary.Array_Remove` (`self.Quests`) QuestIndex))

(fn `ActionIdIsExpected`
  (params (Action :type "/Game/03_Blueprints/Quest/EActionType Enum" :default "NewEnumerator0") (ActionId :type String))
  (returns (Expected :type Boolean) (QuestIndex :type Integer))
  (for (_array_element _array_index) (`self.Quests`)
    (bind ((`Type_2_86DC646144700A12C04818AA1D21B893` _type) (`Id_5_617C013D4E997D033E706682BD127BB1` _id)) (break `/Game/03_Blueprints/Quest/SQuestStep` (`.CurrentStep_9_67AAE3184F891163F26BC0AE25D37C21` (break `/Game/03_Blueprints/Quest/SQuestWrapper` _array_element))))
    (if (and (`|EnumEquality` _type (`local.Action`)) (`KismetStringLibrary.EqualEqual_StrStr` _id (`local.ActionId`)))
      (return true _array_index)))
  (return false -1))

(fn `FindInteractGoal`
  (params (Id :type String))
  (returns (SpheresToGo :type "Array of /Game/03_Blueprints/BP_InteractionBase Object Reference"))
  (locals (AllObjects :type "Array of /Game/03_Blueprints/BP_InteractionBase Object Reference"))
  (bind _outactors (`GameplayStatics.GetAllActorsOfClass` "/Game/03_Blueprints/BP_InteractionBase.BP_InteractionBase_C"))
  (for _array_element _outactors
    (if (`KismetStringLibrary.EqualEqual_StrStr` (`/Game/03_Blueprints/BP_InteractionBase.Id` _array_element) (`local.Id`))
      (`KismetArrayLibrary.Array_Add` (`local.AllObjects`) _array_element)))
  (return (`local.AllObjects`)))

(fn `FindMoveToGoal`
  (params (Id :type String))
  (returns (SpheresToGo :type "Array of /Game/03_Blueprints/Quest/SphereToGo Object Reference"))
  (locals (AllObjects :type "Array of /Game/03_Blueprints/Quest/SphereToGo Object Reference"))
  (bind _outactors (`GameplayStatics.GetAllActorsOfClass` "/Game/03_Blueprints/Quest/SphereToGo.SphereToGo_C"))
  (for _array_element _outactors
    (if (`KismetStringLibrary.EqualEqual_StrStr` (`/Game/03_Blueprints/Quest/SphereToGo.id` _array_element) (`local.Id`))
      (`KismetArrayLibrary.Array_Add` (`local.AllObjects`) _array_element)))
  (return (`local.AllObjects`)))

(fn `ProgressQuest`
  (params (QuestIndex :type Integer))
  (returns (Finished :type Boolean))
  (bind (_quest _currentstepindex _currentstep) (break `/Game/03_Blueprints/Quest/SQuestWrapper` (`|GetArrayItem` (`self.Quests`) (`local.QuestIndex`))))
  (bind ((`CurrentStep_9_67AAE3184F891163F26BC0AE25D37C21` _currentstep_2) (`CurrentActionNumber_15_38B18BB241762E7FA889C8A4D26732CA` _currentactionnumber)) (break `/Game/03_Blueprints/Quest/SQuestWrapper` (`|GetArrayItem` (`self.Quests`) (`local.QuestIndex`))))
  (bind ((`CurrentStep_9_67AAE3184F891163F26BC0AE25D37C21` _currentstep_3) (`CurrentActionNumber_15_38B18BB241762E7FA889C8A4D26732CA` _currentactionnumber_2)) (break `/Game/03_Blueprints/Quest/SQuestWrapper` (`|GetArrayItem` (`self.Quests`) (`local.QuestIndex`))))
  (bind ((`TextForPlayer_7_0AF38C0D4441331E1301D69330518E34` _textforplayer) (`ActionNumber_17_44DC010742E5685B013B38A6CF78019C` _actionnumber)) (break `/Game/03_Blueprints/Quest/SQuestStep` _currentstep_3))
  (bind _returnvalue (+ _currentstepindex 1))
  (bind _steps (`/Game/03_Blueprints/Quest/BP_DA_Quest.Steps` _quest))
  (if (<= (`.ActionNumber_17_44DC010742E5685B013B38A6CF78019C` (break `/Game/03_Blueprints/Quest/SQuestStep` _currentstep_2)) (+ _currentactionnumber 1))
    (`self.UnbindStep` _currentstep)
    (`KismetSystemLibrary.PrintString` (`KismetStringLibrary.Concat_StrStr` "Task Completed :" (`.TextForPlayer_7_0AF38C0D4441331E1301D69330518E34` (break `/Game/03_Blueprints/Quest/SQuestStep` _currentstep))) true true (struct :`R` 1.0 :`G` 0.666213 :`B` 0.302083 :`A` 1.0) 5.0)
    (if (<= (`KismetArrayLibrary.Array_Length` _steps) _returnvalue)
      (return true)
      (else
        (`KismetArrayLibrary.Array_Set` (`self.Quests`) (`local.QuestIndex`) (make `/Game/03_Blueprints/Quest/SQuestWrapper` _quest _returnvalue (`|GetArrayItem` _steps _returnvalue)))
        (`self.NextStep` (`.CurrentStep_9_67AAE3184F891163F26BC0AE25D37C21` (break `/Game/03_Blueprints/Quest/SQuestWrapper` (`|GetArrayItem` (`self.Quests`) (`local.QuestIndex`)))))
        (return false)))
    (else
      (`/Engine/EditorBlueprintResources/StandardMacros.IncrementInt` _currentactionnumber
        (:`  `
          (`KismetSystemLibrary.PrintString` (`KismetStringLibrary.Concat_StrStr` _textforplayer " : " (`KismetStringLibrary.Conv_IntToString` _currentactionnumber_2) " / " (`KismetStringLibrary.Conv_IntToString` _actionnumber))))))))