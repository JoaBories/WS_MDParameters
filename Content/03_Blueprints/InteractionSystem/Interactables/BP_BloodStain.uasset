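; BP_BloodStain is an interactable blood stain that the player can clean away.
; It caches the player character on BeginPlay, then on Interact plays the AM_Balai montage on that character's mesh.
; The stain destroys itself as soon as the montage call fires, without waiting for completion.
; Interaction getters supply the fixed prompt, type, hold duration, tap count and location.
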(event `self.ReceiveBeginPlay`
  (bind _asbp_third_person_character (cast `/Game/03_Blueprints/BP_ThirdPersonCharacter` (`GameplayStatics.GetPlayerCharacter` 0)))
  (set `self.Chara Ref` _asbp_third_person_character))

(event `/Game/03_Blueprints/InteractionSystem/BPI_Interactable.Interact`
  (params (Interactor :type "Actor Object Reference"))
  (`|PlayMontage` (`Character.Mesh` (`self.Chara Ref`)) "/Game/06_Animation/AM_Balai.AM_Balai"
    (:`then`
      (`self.K2_DestroyActor`))))

(fn `GetHoldDuration`
  (returns (Duration :type "Float (double-precision)"))
  (return 1.0))

(fn `GetInteractionLocation`
  (returns (`Location ` :type "Vector Structure"))
  (return (0.0 0.0 0.0)))

(fn `GetInteractionPrompt`
  (returns (Value :type Text))
  (return "to clean"))

(fn `GetInteractionType`
  (returns (Type :type "/Game/03_Blueprints/InteractionSystem/E_InteractionTypes Enum"))
  (return "NewEnumerator0"))

(fn `GetTapCount`
  (returns (Value :type Integer))
  (return 0))

(fn `UserConstructionScript`)