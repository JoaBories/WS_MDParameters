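; BP_Chest is an interactable chest whose lid swings when the player interacts with it.
; Interact plays a Timeline whose Alpha track directly sets the Lid's relative roll, with no reverse path for closing.
; The interaction getters return default values: the first interaction type, an empty prompt, a zero location, and zero hold duration and tap count.
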(event `/Game/03_Blueprints/InteractionSystem/BPI_Interactable.Interact`
  (params (Interactor :type "Actor Object Reference"))
  (bind (_direction _alpha) (`Timeline|Timeline`)
    (:`Update`
      (`SceneComponent.K2_SetRelativeRotation` (`self.Lid`) (`KismetMathLibrary.MakeRotator` _alpha) false false))))

(fn `GetHoldDuration`
  (returns (Duration :type "Float (double-precision)"))
  (return 0.0))

(fn `GetInteractionLocation`
  (returns (`Location ` :type "Vector Structure"))
  (return (0.0 0.0 0.0)))

(fn `GetInteractionPrompt`
  (returns (Value :type Text))
  (return ""))

(fn `GetInteractionType`
  (returns (Type :type "/Game/03_Blueprints/InteractionSystem/E_InteractionTypes Enum"))
  (return "NewEnumerator0"))

(fn `GetTapCount`
  (returns (Value :type Integer))
  (return 0))

(fn `UserConstructionScript`)