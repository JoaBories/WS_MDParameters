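; BP_Ladder is an interactable ladder that stays dormant until it is activated under the "Ladder" ID.
; BeginPlay caches the third-person game mode, disables the Sphere's collision and hides the Niagara effect.
; Activate enables query collision, shows the effect and applies a gold outline overlay material to the mesh.
; Interact hands off to the game mode's ladder fade-to-black, so the Blueprint contains no climbing logic.
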(event `self.ReceiveBeginPlay`
  (bind _asbp_third_person_game_mode (cast `/Game/03_Blueprints/BP_ThirdPersonGameMode` (`GameplayStatics.GetGameMode`)))
  (set `self.As BP Third Person Game Mode` _asbp_third_person_game_mode)
  (`PrimitiveComponent.SetCollisionEnabled` (`self.Sphere`) "NoCollision")
  (`SceneComponent.SetVisibility` (`self.Niagara`) false false))

(event `/Game/03_Blueprints/InteractionSystem/BPI_Interactable.Interact`
  (params (Interactor :type "Actor Object Reference"))
  (`/Game/03_Blueprints/BP_ThirdPersonGameMode.PlayFadeBlackLadder` (`self.As BP Third Person Game Mode`)))

(event `/Game/03_Blueprints/Quest/BPI_QuestActivatable.Activate`
  (`PrimitiveComponent.SetCollisionEnabled` (`self.Sphere`) "QueryOnly")
  (`SceneComponent.SetVisibility` (`self.Niagara`) true false)
  (`MeshComponent.SetOverlayMaterial` (`self.StaticMesh`) "/Game/02_Materials/MI_OutlineGold.MI_OutlineGold"))

(fn `GetActivatableId`
  (returns (Id :type String))
  (return "Ladder"))

(fn `GetHoldDuration`
  (returns (Duration :type "Float (double-precision)"))
  (return 0.0))

(fn `GetInteractionLocation`
  (returns (`Location ` :type "Vector Structure"))
  (return (0.0 0.0 0.0)))

(fn `GetInteractionPrompt`
  (returns (Value :type Text))
  (return ""))

(fn `GetInteractionType`
  (returns (Type :type "/Game/03_Blueprints/InteractionSystem/E_InteractionTypes Enum"))
  (return "NewEnumerator0"))

(fn `GetTapCount`
  (returns (Value :type Integer))
  (return 0))

(fn `UserConstructionScript`)