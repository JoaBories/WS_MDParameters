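; BP_NPC is an interactable NPC in the interaction system, offering a "to talk" prompt.
; It supplies the interaction type, zero hold duration and tap count, and a prompt position taken from its InteractionLocation component.
; On Interact it snaps its yaw to face the interactor and plays a sound at its location; no dialogue logic is present.
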(event `/Game/03_Blueprints/InteractionSystem/BPI_Interactable.Interact`
  (params (Interactor :type "Actor Object Reference"))
  (bind (_returnvalue_roll _returnvalue_pitch _returnvalue_yaw) (`KismetMathLibrary.BreakRotator` (`KismetMathLibrary.FindLookAtRotation` (`self.K2_GetActorLocation`) (`self.K2_GetActorLocation` Interactor))))
  (`self.K2_SetActorRotation` (`KismetMathLibrary.MakeRotator` 0.0 0.0 _returnvalue_yaw))
  (`GameplayStatics.PlaySoundAtLocation` "/Engine/VREditor/Sounds/UI/Object_Snaps_To_Another_Actor.Object_Snaps_To_Another_Actor" (`self.K2_GetActorLocation`) (struct) 1.0 1.0 0.0 null null null null))

(fn `GetHoldDuration`
  (returns (Duration :type "Float (double-precision)"))
  (return 0.0))

(fn `GetInteractionLocation`
  (returns (`Location ` :type "Vector Structure"))
  (return (`SceneComponent.K2_GetComponentLocation` (`self.InteractionLocation`))))

(fn `GetInteractionPrompt`
  (returns (Value :type Text))
  (return "to talk"))

(fn `GetInteractionType`
  (returns (Type :type "/Game/03_Blueprints/InteractionSystem/E_InteractionTypes Enum"))
  (return "NewEnumerator0"))

(fn `GetTapCount`
  (returns (Value :type Integer))
  (return 0))

(fn `UserConstructionScript`)