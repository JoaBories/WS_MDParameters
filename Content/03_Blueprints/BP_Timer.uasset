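; BP_Timer is a countdown actor that starts a looping timer on BeginPlay.
; Every tenth of a second TickTimer lowers the Timer variable and prints it to screen.
; At zero or below it prints "Dead" but never clears the timer, so the countdown keeps running negative.
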(event `self.ReceiveBeginPlay`
  (`self.LaunchTimer`))

(event `LaunchTimer`
  (`KismetSystemLibrary.K2_SetTimerDelegate` (delegate `TickTimer`) 0.1 true true))

(event `TickTimer`
  (bind _output_get (set `self.Timer` (- (`self.Timer`) 0.1)))
  (`KismetSystemLibrary.PrintString` (`KismetStringLibrary.Conv_DoubleToString` _output_get))
  (if (<= (`self.Timer`) 0.0)
    (`KismetSystemLibrary.PrintString` "Dead")))

(fn `UserConstructionScript`)