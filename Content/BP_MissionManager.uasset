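; BP_MissionManager runs a linear quest, stepping through the Quest array from BeginPlay and printing objective, success and finish text.
; For "Move to" steps, NextStep finds SphereToGo actors with a matching Id and binds MoveTo to their OnReachedByPlayer event.
; MoveTo checks the Id, unbinds from the current sphere, increments the index and either calls NextStep or ends the quest.
; Interact and Dialogue handlers are empty stubs.
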(event `self.ReceiveBeginPlay`
  (`self.NextStep`))

(event `Interact`
  (params (id :type String))
  (if (`KismetStringLibrary.EqualEqual_StrStr` id)
    _))

(event `Dialogue`
  (params (id :type String))
  (if (`KismetStringLibrary.EqualEqual_StrStr` id)
    _))

(event `NextStep`
  (bind (_type _id _textforplayer) (break `/Game/QuestStep` (`|GetArrayItem` (`self.Quest`) (`self.current`))))
  (switch `/Game/ActionType` _type
    (:`NewEnumerator0`
      (bind _outactors (`GameplayStatics.GetAllActorsOfClass` "/Game/SphereToGo.SphereToGo_C"))
      (for _array_element _outactors
        (if (`KismetStringLibrary.EqualEqual_StrStr` (`/Game/SphereToGo.id` _array_element) _id)
          (bind _output_get (set `self.CurrentSphere` _array_element))
          (add `/Game/SphereToGo.OnReachedByPlayer` _output_get (delegate `MoveTo`))
          (`KismetSystemLibrary.PrintString` _textforplayer))))))

(event `MoveTo`
  (params (Id :type String))
  (bind (_type _id _textforplayer) (break `/Game/QuestStep` (`|GetArrayItem` (`self.Quest`) (`self.current`))))
  (if (`KismetStringLibrary.EqualEqual_StrStr` Id _id)
    (`KismetSystemLibrary.PrintString` (`KismetStringLibrary.Concat_StrStr` _textforplayer "Success"))
    (remove `/Game/SphereToGo.OnReachedByPlayer` (`self.CurrentSphere`) (delegate `MoveTo`))
    (bind _result (`/Engine/EditorBlueprintResources/StandardMacros.IncrementInt` (`self.current`))
      (:`  `
        (if (>= _result (`KismetArrayLibrary.Array_Length` (`self.Quest`)))
          (`KismetSystemLibrary.PrintString` "Finish Quest")
          (else
            (`self.NextStep`)))))))

(fn `UserConstructionScript`)